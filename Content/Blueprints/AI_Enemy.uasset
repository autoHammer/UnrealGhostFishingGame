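; AI_Enemy is an enemy character that sways back and forth and opens the game-over map when anything overlaps its Box component.
; Tick drives it from an accumulated timer: one sine wave flips its rotation by 180 degrees, and a faster one scales forward movement input.
; The start position is saved on BeginPlay, but only unused distance-check nodes read it.
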(event OnComponentBeginOverlap(Box)
  (params (OverlappedComponent :type Primitive%20Component%20Object%20Reference) (OtherActor :type Actor%20Object%20Reference) (OtherComp :type Primitive%20Component%20Object%20Reference) (OtherBodyIndex :type Integer) (bFromSweep :type Boolean) (SweepResult :type Hit%20Result%20Structure%20%28by%20ref%29))
  (Game|OpenLevel(byObjectReference) "/Game/Level/Map_GameOver.Map_GameOver"))

(event EventBeginPlay
  (Variables|Default|SetStartPosX (Transformation|GetActorLocation)))

(event Collision|EventActorBeginOverlap
  (params (OtherActor :type Actor%20Object%20Reference)))

(event EventTick
  (params (DeltaSeconds :type Float%20%28single-precision%29))
  (bind _output_get (Variables|Default|SetTimer (+ (Variables|Default|GetTimer) (Utilities|Time|GetWorldDeltaSeconds))))
  (if (>= (Math|Trig|Sin(Degrees) (* _output_get 5e+01)) -0.01)
    (Transformation|SetActorRotation "0, 0, 0")
    (else
      (Transformation|SetActorRotation "0.000000,180.000000,0.000000")))
  (Pawn|Input|AddMovementInput (Transformation|GetActorForwardVector) (Math|Trig|Sin(Degrees) (* _output_get 1e+02)) false))

(fn ConstructionScript)